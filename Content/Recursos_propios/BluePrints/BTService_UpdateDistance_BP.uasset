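; Behavior tree service that keeps the Distance blackboard key updated with how far the AI-controlled NPC is from its target.
; On each tick it casts the owner to AIController and reads the controlled pawn's location and the Target actor's location from the blackboard.
; It writes their horizontal 2D distance, ignoring height, to the Distance key as a float.
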(event EventTick
  (params (OwnerActor :type Actor%20Object%20Reference) (DeltaSeconds :type Float%20%28single-precision%29))
  ;[1 1 1] Primero obtengo la localización del NPC (controlado por AIcontroller), luego la del jugador, calculo la distancia entre ambas localizaciones con un vector 2d y después se lo asigno a la variable Distance del blackboard
  (bind _asaicontroller (Utilities|Casting|CastToAIController OwnerActor))
  (Class|BTFunctionLibrary|SetBlackboardValueasFloat (Variables|Default|GetDistance) (Math|Vector|Distance2D(Vector) (Math|Conversions|ToVector2D(Vector) (Transformation|GetActorLocation (Pawn|GetControlledPawn _asaicontroller))) (Math|Conversions|ToVector2D(Vector) (Transformation|GetActorLocation (AI|BehaviorTree|GetBlackboardValueasActor (Variables|Default|GetTarget)))))))